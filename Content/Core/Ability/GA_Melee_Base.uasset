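; GA_Melee_Base is a base Gameplay Ability for melee combo attacks that deal damage to traced targets.
; Combo start plays the attack montage, then ends the ability after the attack-time delay and a two-way net sync.
; Melee montage events trigger a hitscan trace only when locally controlled, and the result is sent as target data.
; When that data is ready, a damage GameplayEffect with SetByCaller magnitude is applied to the targets.
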(event `self.OnComboStart`
  (`AbilityTask_PlayMontageAndWaitForEvent.PlayMontageAndWaitForEvent` "None" (`self.Attack Montage`) (struct :`GameplayTags` (struct :`(TagName` "Event.Melee"))) 1.0 "None" false
    (:`then`
      (`AbilityTask_WaitDelay.WaitDelay` (`self.Attack Time`)
        (:`OnFinish`
          (`AbilityTask_NetworkSyncPoint.WaitNetSync` "BothWait"
            (:`OnSync`
              (`self.K2_EndAbility`))))))
    (:`EventReceived`
      (`self.IsLocallyControlled` ; Server 側でも実行するか検討
        (:`True`
          (`self.Targeting`))))))

(event `Targeting`
  (bind (_asynctaskproxy _intargetdata) (`AbilityTask_CreateTargetDataByMeleeHitscan.CreateCreateTargetDataByMeleeHitscan` :`InObjectTypes` (`self.Trace Object Types`) :`InCollisionChannel` "ECC_Pawn" :`InDuration` (`self.Trace Duration`) :`InRadius` (`self.Trace Radius`) :`InDistance` (`self.Trace Distance`))
    (:`OnCreated`
      (`self.SendTargetData` _intargetdata))))

(event `self.OnTargetDataReady`
  (params (TargetData :type "GameplayAbilityTargetDataHandle Structure (by ref)"))
  (bind _returnvalue (`AbilitySystemBlueprintLibrary.AssignTagSetByCallerMagnitude` (`self.MakeOutgoingGameplayEffectSpec` (`self.Damage GE`)) (struct :`TagName` "SetByCaller.Magnitude") (`self.Damage`)))
  (`self.K2_ApplyGameplayEffectSpecToTarget` _returnvalue TargetData))