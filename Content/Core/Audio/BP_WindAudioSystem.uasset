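; BP_WindAudioSystem drives the AmbientWind audio parameters from the player pawn's speed and surroundings.
; Outdoors, a looping MultiGate spreads five world-axis visibility traces (up, left, right, forward, back) across ticks, one per tick.
; Each hit lowers Wind on the next cycle, while left and right hit distances set the pan parameters.
; When not exterior, Wind follows the clamped speed value, which also always feeds PawnSpeed.
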(event `self.ReceiveTick`
  (params (DeltaSeconds :type "Float (single-precision)"))
  (bind _returnvalue (`GameplayStatics.GetPlayerPawn` 0))
  (bind _tracedistance (`self.TraceDistance`))
  (bind _ambientwind (`self.AmbientWind`))
  (`/Engine/EditorBlueprintResources/StandardMacros.IsValid` _returnvalue
    (:`Is Valid`
      (set `self.PawnLoc` (`self.K2_GetActorLocation` _returnvalue))
      (`KismetArrayLibrary.Array_Set` (`self.Player`) 0 _returnvalue)
      (bind _output_get (set `self.Speed` (`KismetMathLibrary.MapRangeClamped` (`KismetMathLibrary.VSize` (`self.GetVelocity` _returnvalue)) 600.0 2500.0 0.0 1.0)))
      (`AudioParameterControllerInterface.SetFloatParameter` (`self.AmbientWind`) "PawnSpeed" _output_get)
      (if (`self.IsExterior`)
        (`|MultiGate` false true
          (:`Out 0`
            (bind _output_get_2 (set `self.Wind` (- 1.0 (* (`KismetMathLibrary.Conv_IntToDouble` (`self.Hits`)) 0.2))))
            (`AudioParameterControllerInterface.SetFloatParameter` (`self.AmbientWind`) "Wind" _output_get_2)
            (set `self.Hits` 0)
            (`self.GetTrace` (0.0 0.0 1.0)))
          (:`Out 1`
            (bind _distance (`self.GetTrace` (0.0 -1.0 0.0))) ; Left
            (`AudioParameterControllerInterface.SetFloatParameter` _ambientwind "Pan.L" (`KismetMathLibrary.SafeDivide` _distance _tracedistance)))
          (:`Out 2`
            (bind _distance_2 (`self.GetTrace` (0.0 1.0 0.0))) ; Right
            (`AudioParameterControllerInterface.SetFloatParameter` _ambientwind "Pan.R" (`KismetMathLibrary.SafeDivide` _distance_2 _tracedistance)))
          (:`Out 3`
            (`self.GetTrace` (1.0 0.0 0.0)) ; Forward
          )
          (:`Out 4`
            (`self.GetTrace` (-1.0 0.0 0.0)) ; Back
          ))
        (else
          (`AudioParameterControllerInterface.SetFloatParameter` (`self.AmbientWind`) "Wind" (`self.Speed`)))))))

(fn `UserConstructionScript`)